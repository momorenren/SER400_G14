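; Drill station start button actor that begins the drill sequence when any actor overlaps it.
; The overlap plays two timed 2D voice or sound cues (attach, then stand clear), then broadcasts StartDrillBtnMessage to every actor implementing the StartBtn_BP interface.
; A RunOnce flag, set only after both delays finish, blocks later triggers until ResetDrillStation clears it.
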(event EventBeginPlay)

(event Collision|EventActorBeginOverlap
  (params (OtherActor :type Actor%20Object%20Reference))
  (if (not (Variables|Default|GetrunOnce))
    (Audio|PlaySound2D "/Game/G14_Assect/sfx/attachActor.attachActor" 1.0 1.0 0.0 0 0)
    (Utilities|FlowControl|Delay 0.8)
    (Audio|PlaySound2D "/Game/drill/sfx/standClear.standClear" 1.0 1.0 0.0 0 0)
    (Utilities|FlowControl|Delay 3.5)
    (Variables|Default|SetrunOnce true)
    (bind _outactors (Actor|GetAllActorswithInterface "/Game/drill/startBtn/startBtn_BP.startBtn_BP_C"))
    (Class|StartBtnBP|StartDrillBtn(Message) _outactors)))

(event EventTick
  (params (DeltaSeconds :type Float%20%28single-precision%29)))

(event EventResetDrillStation
  (Variables|Default|SetrunOnce false))

(fn ConstructionScript)