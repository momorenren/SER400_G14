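; Blueprint for a PCB actor, apparently one piece in a station-based process with a UV mesh and collider.
; On collider overlap it passes itself to the other actor via TakePcbMessage and sends reset message 2 to all StationActivate actors.
; Events show, hide or reset the mesh to its BeginPlay transform.
; SetPcbState stores a state, but GetPcbState returns a fixed enum value and GivePcb is empty.
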(event OnComponentBeginOverlap(PCB_UV_collider)
  (params (OverlappedComponent :type Primitive%20Component%20Object%20Reference) (OtherActor :type Actor%20Object%20Reference) (OtherComp :type Primitive%20Component%20Object%20Reference) (OtherBodyIndex :type Integer) (bFromSweep :type Boolean) (SweepResult :type Hit%20Result%20Structure%20%28by%20ref%29))
  (Class|PcbInterface|TakePcb(Message) OtherActor self)
  (bind _outactors (Actor|GetAllActorswithInterface "/Game/pcb/stationActivate.stationActivate_C"))
  (Class|StationActivate|ResetStationResets(Message) _outactors 2))

(event EventBeginPlay
  (Variables|Default|SetorigLocation (Transformation|GetWorldTransform (Variables|Default|GetStaticMeshUV))))

(event EventResetUV
  (bind _staticmeshuv (Variables|Default|GetStaticMeshUV))
  (Transformation|SetWorldTransform _staticmeshuv (Variables|Default|GetorigLocation) false false)
  (Rendering|SetVisibility _staticmeshuv true false))

(event EventSetPcbState
  (params (set%20state :type pcb_state%20Enum :default "NewEnumerator0"))
  (Variables|Default|Setthis_pcb_state set%20state))

(event EventHide
  (Rendering|SetVisibility (Variables|Default|GetStaticMeshUV) false false))

(event EventPcb2Show
  (Rendering|SetVisibility (Variables|Default|GetStaticMeshUV) true false))

(fn ConstructionScript)

(fn GivePcb
  (return 0))

(fn GetPcbState
  (return "NewEnumerator0"))