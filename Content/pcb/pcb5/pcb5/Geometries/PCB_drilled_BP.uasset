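; PCB_drilled_BP is the drilled PCB actor, which is shown, hidden and reset as part of a drill station.
; It caches the mesh's world transform on BeginPlay and hides it in game when its collider overlaps a PCB_holderBP.
; Pcb5Show makes the mesh visible, while ResetDrillStation makes it invisible and restores the cached transform.
; Neither event clears the hidden-in-game flag set by the overlap.
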(event OnComponentBeginOverlap(PCB_drill_collider)
  (params (OverlappedComponent :type Primitive%20Component%20Object%20Reference) (OtherActor :type Actor%20Object%20Reference) (OtherComp :type Primitive%20Component%20Object%20Reference) (OtherBodyIndex :type Integer) (bFromSweep :type Boolean) (SweepResult :type Hit%20Result%20Structure%20%28by%20ref%29))
  (Utilities|Casting|CastToPCB_holderBP OtherActor)
  (Development|SetHiddeninGame (Variables|Default|GetPCB_drilled_SM) true false))

(event EventBeginPlay
  ;[1 1 1] Initialise
  (Variables|Default|SetorigLocation (Transformation|GetWorldTransform (Variables|Default|GetPCB_drilled_SM))))

(event Collision|EventActorBeginOverlap
  (params (OtherActor :type Actor%20Object%20Reference)))

(event EventTick
  (params (DeltaSeconds :type Float%20%28single-precision%29)))

(event EventPcb5Show
  (Rendering|SetVisibility (Variables|Default|GetPCB_drilled_SM) true true))

(event EventResetDrillStation
  (bind _pcb_drilled_sm (Variables|Default|GetPCB_drilled_SM))
  (Rendering|SetVisibility _pcb_drilled_sm false false)
  (Transformation|SetWorldTransform _pcb_drilled_sm (Variables|Default|GetorigLocation) false false))

(fn ConstructionScript)