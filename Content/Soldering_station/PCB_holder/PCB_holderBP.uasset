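; PCB holder at the soldering station that runs the drill-to-holder and soldering steps of a staged soldering task.
; Overlaps with the drilled plate and the soldering iron advance a step enum, swapping the held PCB for the components board after a timed solder delay.
; Interface broadcasts update instruction text, and share the enum after soldering and on reset.
; A reset event hides both boards and returns to the drill-to-holder step.
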(event OnComponentBeginOverlap(PCB_holder_collider)
  (params (OverlappedComponent :type Primitive%20Component%20Object%20Reference) (OtherActor :type Actor%20Object%20Reference) (OtherComp :type Primitive%20Component%20Object%20Reference) (OtherBodyIndex :type Integer) (bFromSweep :type Boolean) (SweepResult :type Hit%20Result%20Structure%20%28by%20ref%29))
  (bind _solder_timer_var (Variables|Default|GetSolder_timer_var))
  (bind _solder_timer_var_2 (Variables|Default|GetSolder_timer_var))
  ;[0.121 0.6366 1] Iron overlaps holder
  (Utilities|Casting|CastToSoldering_IronBP OtherActor)
  (switch Utilities|FlowControl|Switch|SwitchonSolder_Step_Enum (Variables|Default|GetSolder_enum_var)
    (:NewEnumerator1
      (Actor|Tick|SetActorTickEnabled _solder_timer_var true)
      (Rendering|SetActorHiddenInGame _solder_timer_var false)
      (Utilities|FlowControl|Delay 3.5)
      (Rendering|SetActorHiddenInGame _solder_timer_var_2 true)
      (Actor|Tick|SetActorTickEnabled _solder_timer_var_2)
      (Development|SetHiddeninGame (Variables|Default|Getpcb5) true false)
      (Rendering|SetActorHiddenInGame (Variables|Default|GetPCB_components_board) false)
      (bind _outactors (Actor|GetAllActorswithInterface "/Game/Soldering_station/Solder_text/solder_text_interface.solder_text_interface_C"))
      (Class|SolderTextInterface|IronHide(Message) _outactors)
      (Class|SolderTextInterface|TestBoardShow(Message) _outactors)
      (Variables|Default|SetSolder_enum_var "NewEnumerator2")
      (bind _outactors_2 (Actor|GetAllActorswithInterface "/Game/Soldering_station/Solder_station_enum/Solder_Enum_Var_pass_BPinterface.Solder_Enum_Var_pass_BPinterface_C"))
      (Class|SolderEnumVarPassBPinterface|SolderEnumPass(Message) _outactors_2 (Variables|Default|GetSolder_enum_var)))))

(event OnComponentBeginOverlap(Holder_Whole_collider)
  (params (OverlappedComponent :type Primitive%20Component%20Object%20Reference) (OtherActor :type Actor%20Object%20Reference) (OtherComp :type Primitive%20Component%20Object%20Reference) (OtherBodyIndex :type Integer) (bFromSweep :type Boolean) (SweepResult :type Hit%20Result%20Structure%20%28by%20ref%29))
  ;[1 0.2555 0.5789] PCB from drill overlaps with PCB holder
  (Utilities|Casting|CastToPCB_drill_plate_BP OtherActor)
  (switch Utilities|FlowControl|Switch|SwitchonSolder_Step_Enum (Variables|Default|GetSolder_enum_var)
    (:NewEnumerator0
      (Audio|Components|Audio|Play (Variables|Default|Getholder_PCB_audio) 0.0)
      (Development|SetHiddeninGame (Variables|Default|Getpcb5) false false)
      (bind _outactors (Actor|GetAllActorswithInterface "/Game/Soldering_station/Solder_text/solder_text_interface.solder_text_interface_C"))
      (Class|SolderTextInterface|IronShow(Message) _outactors)
      (Class|SolderTextInterface|DrillMovetoSolderHide(Message) _outactors)
      (Variables|Default|SetSolder_enum_var "NewEnumerator1"))))

(event EventResetSoldering
  ;[0.09945 1 0.5523] Reset soldering station
  (Development|SetHiddeninGame (Variables|Default|Getpcb5) true false)
  (Rendering|SetActorHiddenInGame (Variables|Default|GetPCB_components_board) true)
  (bind _outactors (Actor|GetAllActorswithInterface "/Game/Soldering_station/Solder_text/solder_text_interface.solder_text_interface_C"))
  (Class|SolderTextInterface|ProjectorHide(Message) _outactors)
  (Class|SolderTextInterface|TestBoardHide(Message) _outactors)
  (Class|SolderTextInterface|IronHide(Message) _outactors)
  (Class|SolderTextInterface|DrillMovetoSolderHide(Message) _outactors)
  (bind _output_get (Variables|Default|SetSolder_enum_var "NewEnumerator0"))
  (bind _outactors_2 (Actor|GetAllActorswithInterface "/Game/Soldering_station/Solder_station_enum/Solder_Enum_Var_pass_BPinterface.Solder_Enum_Var_pass_BPinterface_C"))
  (Class|SolderEnumVarPassBPinterface|SolderEnumPass(Message) _outactors_2 _output_get))

(event EventBeginPlay
  ;[1 1 1] Initial
  (bind _returnvalue (Actor|GetActorOfClass "/Game/Chemical_station/Timer_display/Timer_solder_BP.Timer_solder_BP_C"))
  (bind _output_get (Variables|Default|SetSolder_timer_var _returnvalue))
  (Utilities|Casting|CastToTimer_solder_BP _output_get)
  (Rendering|SetActorHiddenInGame (Variables|Default|GetSolder_timer_var) true)
  (Actor|Tick|SetActorTickEnabled (Variables|Default|GetSolder_timer_var))
  (bind _returnvalue_2 (Actor|GetActorOfClass "/Game/Soldering_station/PCB_compoents_BP.PCB_compoents_BP_C"))
  (bind _output_get_2 (Variables|Default|SetPCB_components_board _returnvalue_2))
  (Utilities|Casting|CastToPCB_compoents_BP _output_get_2)
  (Rendering|SetActorHiddenInGame (Variables|Default|GetPCB_components_board) true)
  (Development|SetHiddeninGame (Variables|Default|Getpcb5) true false))

(fn ConstructionScript)