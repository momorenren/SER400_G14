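; PCB drill plate Blueprint for the soldering station, showing a PCB mesh that disappears when the PCB holder reaches it.
; On BeginPlay it caches the PCB's world transform.
; Overlap of its box with a PCB_holderBP hides the PCB mesh.
; The ResetSoldering event teleport-free restores the saved transform and makes the PCB visible again.
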(event OnComponentBeginOverlap(Box)
  (params (OverlappedComponent :type Primitive%20Component%20Object%20Reference) (OtherActor :type Actor%20Object%20Reference) (OtherComp :type Primitive%20Component%20Object%20Reference) (OtherBodyIndex :type Integer) (bFromSweep :type Boolean) (SweepResult :type Hit%20Result%20Structure%20%28by%20ref%29))
  (Utilities|Casting|CastToPCB_holderBP OtherActor)
  (Development|SetHiddeninGame (Variables|Default|Getpcb5) true false))

(event EventBeginPlay
  (Variables|Default|Settrans_plate_PCB (Transformation|GetWorldTransform (Variables|Default|Getpcb5))))

(event Collision|EventActorBeginOverlap
  (params (OtherActor :type Actor%20Object%20Reference)))

(event EventTick
  (params (DeltaSeconds :type Float%20%28single-precision%29)))

(event EventResetSoldering
  (Transformation|SetWorldTransform (Variables|Default|Getpcb5) (Variables|Default|Gettrans_plate_PCB) false false)
  (Development|SetHiddeninGame (Variables|Default|Getpcb5) false false))

(fn ConstructionScript)