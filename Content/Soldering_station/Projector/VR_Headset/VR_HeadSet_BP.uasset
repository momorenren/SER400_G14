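; VR headset prop in the soldering station that acts as a one-time trigger to end the level.
; An underwater sound plays from BeginPlay until a VRPawn first overlaps the headset collider, guarded by a boolean.
; That touch hides the headset's 3D text, reveals a poster, text renders and spotlight, and swaps the audio to wake-up music.
; After a fixed delay, it opens the endMap level.
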(event OnComponentBeginOverlap(HeadSet_collider)
  (params (OverlappedComponent :type Primitive%20Component%20Object%20Reference) (OtherActor :type Actor%20Object%20Reference) (OtherComp :type Primitive%20Component%20Object%20Reference) (OtherBodyIndex :type Integer) (bFromSweep :type Boolean) (SweepResult :type Hit%20Result%20Structure%20%28by%20ref%29))
  ;[0.2859 0.1185 1] VR hands touch the headset
  (Utilities|Casting|CastToVRPawn OtherActor)
  ;[1 1 1] Check first touch or touch again
  (if (not (Variables|Default|Getcheck_touch_headset))
    (Variables|Default|Setcheck_touch_headset true)
    ;[0.1459 0.2664 1] Run these tasks
    (Utilities|FlowControl|Sequence
      (:then_0
        (Rendering|SetVisibility (Variables|Default|GetText3D_headset) false false))
      (:then_1
        (Rendering|SetVisibility (Variables|Default|GetPoster) true false))
      (:then_2
        (Rendering|SetVisibility (Variables|Default|GetTextRender) true false))
      (:then_3
        (Rendering|SetVisibility (Variables|Default|GetTextRender1) true false))
      (:then_4
        (Rendering|SetVisibility (Variables|Default|GetTextRender2) true false))
      (:then_5
        (Rendering|SetVisibility (Variables|Default|GetTextRender3) true false))
      (:then_6
        (Rendering|SetVisibility (Variables|Default|GetTextRender4) true false))
      (:then_7
        (Rendering|SetVisibility (Variables|Default|GetTextRender5) true false))
      (:then_8
        (Rendering|SetVisibility (Variables|Default|GetSpotLight) true false))
      (:then_9
        (Audio|Components|Audio|Stop (Variables|Default|Getunder_water))
        (Audio|Components|Audio|Play (Variables|Default|Getwake_up_music_Cue) 0.0)
        (Utilities|FlowControl|Delay 25.0)
        (Game|OpenLevel(byName) "endMap")))))

(event EventBeginPlay
  ;[0.3936 0.3237 1] Initial Headset
  (Audio|Components|Audio|Play (Variables|Default|Getunder_water) 0.0))

(fn ConstructionScript)