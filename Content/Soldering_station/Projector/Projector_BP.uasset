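; Soldering-station projector whose button, when touched by the VR pawn, starts a Niagara fish show and then leaves the level.
; BeginPlay caches the Light_BP actor, which the button overlap messages to toggle the lights while it plays button audio and sends a hide message through Solder_text_interface.
; After a delay, the camera fade starts and testingMap is opened.
; ResetSoldering deactivates the fish effect.
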(event OnComponentBeginOverlap(Projector_Button_collider)
  (params (OverlappedComponent :type Primitive%20Component%20Object%20Reference) (OtherActor :type Actor%20Object%20Reference) (OtherComp :type Primitive%20Component%20Object%20Reference) (OtherBodyIndex :type Integer) (bFromSweep :type Boolean) (SweepResult :type Hit%20Result%20Structure%20%28by%20ref%29))
  ;[0.1487 0.1828 1] VR hands touch the button
  (Utilities|Casting|CastToVRPawn OtherActor)
  ;[0.8015 1 0.3101] Turn off lights and active the show from the projector
  (bind _outactors (Actor|GetAllActorswithInterface "/Game/Soldering_station/Solder_text/solder_text_interface.solder_text_interface_C"))
  (Class|SolderTextInterface|ProjectorHide(Message) _outactors)
  (Components|Activation|SetActive (Variables|Default|GetFish_Niagara_Projector) true false)
  (Audio|Components|Audio|Play (Variables|Default|Getprojector_button_audio) 0.0)
  (Class|LightsControlInterfaceBP|ToggleLights(Message) (Variables|Default|GetLight_actor))
  ;[0.5127 0.2776 1] Fade to another level
  (Utilities|FlowControl|Delay 7.0)
  (CameraFades|StartCameraFade :self (Game|GetPlayerCameraManager 0) :ToAlpha 1.0 :Duration 3.0 :bShouldFadeAudio true)
  (Game|OpenLevel(byName) "testingMap"))

(event EventBeginPlay
  ;[1 0.1507 0.4456] Initial the projector
  (bind _returnvalue (Actor|GetActorOfClass "/Game/Soldering_station/Light/Light_BP.Light_BP_C"))
  (bind _output_get (Variables|Default|SetLight_actor _returnvalue))
  (Utilities|Casting|CastToLight _output_get))

(event EventResetSoldering
  ;[1 0.3209 0.3707] Reset soldering station
  (Components|Activation|SetActive (Variables|Default|GetFish_Niagara_Projector) false false))

(fn ConstructionScript)