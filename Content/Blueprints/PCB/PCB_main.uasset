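; PCB actor that holds a state variable and announces itself to actors entering its UV collider.
; On overlap, it sends itself to the other actor through TakePcbMessage.
; SetPcbState and GetPcbState write and read the state, while GivePcb is an empty stub.
; An unconnected leftover branch would hide the board after a cast to Tong_PCB.
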(event OnComponentBeginOverlap(PCB_UV_collider)
  (params (OverlappedComponent :type Primitive%20Component%20Object%20Reference) (OtherActor :type Actor%20Object%20Reference) (OtherComp :type Primitive%20Component%20Object%20Reference) (OtherBodyIndex :type Integer) (bFromSweep :type Boolean) (SweepResult :type Hit%20Result%20Structure%20%28by%20ref%29))
  (Class|PcbInterface|TakePcb(Message) OtherActor self))

(event EventSetPcbState
  (params (set%20state :type pcb_state%20Enum :default "NewEnumerator0"))
  (Variables|Default|Setthis_pcb_state set%20state))

(fn ConstructionScript)

(fn GivePcb
  (return 0))

(fn GetPcbState
  (return (Variables|Default|Getthis_pcb_state)))