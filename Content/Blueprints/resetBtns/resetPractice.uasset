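; A practice reset button actor that fires when another actor overlaps it, with no filter on the overlapping actor.
; Its Cylinder flashes a blue material for half a second, then switches to a cement material.
; It then broadcasts ResetPracticeMessage to every actor implementing ResetPractice_BPI, decoupling it from what gets reset.
; A delayed chain of 2D sounds follows, named for ending play, picking up a PCB and moving to WShop.
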(event EventBeginPlay)

(event EventTick
  (params (DeltaSeconds :type Float%20%28single-precision%29)))

(event Collision|EventActorBeginOverlap
  (params (OtherActor :type Actor%20Object%20Reference))
  (bind _cylinder (Variables|Default|GetCylinder))
  (Rendering|Material|SetMaterial _cylinder 0 "/Engine/EngineDebugMaterials/VertexColorViewMode_BlueOnly.VertexColorViewMode_BlueOnly")
  (Utilities|FlowControl|Delay 0.5)
  (Rendering|Material|SetMaterial _cylinder 0 "/Game/BluePrints/Soldering_iron/7_sement.7_sement")
  (bind _outactors (Actor|GetAllActorswithInterface "/Game/BluePrints/resetBtns/resetPractice_BPI.resetPractice_BPI_C"))
  (Class|ResetPracticeBPI|ResetPractice(Message) _outactors)
  (Audio|PlaySound2D "/Engine/EditorSounds/GamePreview/EndPlayInEditor.EndPlayInEditor" 1.0 1.0 0.0 0 0)
  (Utilities|FlowControl|Delay 3.0)
  (Audio|PlaySound2D "/Game/G14_Assect/sfx/vo/pickupPCB.pickupPCB" 1.0 1.0 0.0 0 0)
  (Utilities|FlowControl|Delay 5.0)
  (Audio|PlaySound2D "/Game/G14_Assect/sfx/vo/move2WShop.move2WShop" 1.0 1.0 0.0 0 0))

(fn ConstructionScript)