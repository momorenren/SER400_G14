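; VR push button that resets a workshop station, the test bed or practice area, or ends or quits the session.
; Touching it with a hand collider plays a sound, briefly swaps its material, then switches on ResetArea.
; Reset cases broadcast through Blueprint interfaces with audio cues, while session cases fade the camera and open another level.
; A proximity trigger toggles a configurable label that rotates to face the player's head.
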(event OnComponentBeginOverlap(SwitchColider)
  (params (OverlappedComponent :type Primitive%20Component%20Object%20Reference) (OtherActor :type Actor%20Object%20Reference) (OtherComp :type Primitive%20Component%20Object%20Reference) (OtherBodyIndex :type Integer) (bFromSweep :type Boolean) (SweepResult :type Hit%20Result%20Structure%20%28by%20ref%29))
  (bind _switch_colider (Variables|Default|GetSwitch%20Colider))
  (bind _reset_area (Variables|Default|Getreset%20area))
  (bind _cylinder (Variables|Default|GetCylinder))
  ;[1 1 1] Press button things
  (bind _asvrpawn (Utilities|Casting|CastToVRPawn (Game|Player|GetPlayerPawn 0)))
  (if (or (Class|PrimitiveComponent|IsOverlappingComponent _switch_colider (Variables|/Game/VRTemplate/Blueprints/VRPawn.VRPawn_C|GetrightSphereCollider1 _asvrpawn)) (Class|PrimitiveComponent|IsOverlappingComponent _switch_colider (Variables|/Game/VRTemplate/Blueprints/VRPawn.VRPawn_C|GetleftSphereCollider _asvrpawn)))
    (Audio|PlaySound2D "/Engine/EditorSounds/GamePreview/EjectFromPlayer.EjectFromPlayer" 1.0 1.0 0.0 0 0)
    (Rendering|Material|SetMaterial _cylinder 0 "/Engine/EngineDebugMaterials/VertexColorViewMode_BlueOnly.VertexColorViewMode_BlueOnly")
    (Utilities|FlowControl|Delay 1.0)
    (Rendering|Material|SetMaterial _cylinder 0 "/Game/Blueprints/Soldering_iron/7_sement.7_sement")
    (switch Utilities|FlowControl|Switch|Switchonreset_button_area _reset_area
      (:NewEnumerator0
        (bind _outactors (Actor|GetAllActorswithInterface "/Game/Interfaces/reset_interface.reset_interface_C"))
        (Class|ResetInterface|Reset(Message) _outactors _reset_area)
        (Audio|PlaySound2D "/Engine/EditorSounds/GamePreview/EndPlayInEditor.EndPlayInEditor" 1.0 1.0 0.0 0 0)
        (Utilities|FlowControl|Delay 1.0)
        (Audio|PlaySound2D "/Game/G14_Assect/sfx/vo/VO/resetPrinterStation.resetPrinterStation" 1.0 1.0 0.0 0 0))
      (:NewEnumerator1
        (bind _outactors_2 (Actor|GetAllActorswithInterface "/Game/Blueprints/resetBtns/resetUV_BPI.resetUV_BPI_C"))
        (Class|ResetUVBPI|ResetUV(Message) _outactors_2)
        (Audio|PlaySound2D "/Engine/EditorSounds/GamePreview/EndPlayInEditor.EndPlayInEditor" 1.0 1.0 0.0 0 0)
        (Utilities|FlowControl|Delay 1.0)
        (Audio|PlaySound2D "/Game/G14_Assect/sfx/vo/VO/resetUVStation.resetUVStation" 1.0 1.0 0.0 0 0))
      (:NewEnumerator2
        (bind _outactors_3 (Actor|GetAllActorswithInterface "/Game/Blueprints/resetBtns/resetChemical_BPI.resetChemical_BPI_C"))
        (Class|ResetChemicalBPI|ResetChemical(Message) _outactors_3)
        (Audio|PlaySound2D "/Engine/EditorSounds/GamePreview/EndPlayInEditor.EndPlayInEditor" 1.0 1.0 0.0 0 0)
        (Utilities|FlowControl|Delay 1.0)
        (Audio|PlaySound2D "/Game/G14_Assect/sfx/vo/VO/resetChemStation.resetChemStation" 1.0 1.0 0.0 0 0))
      (:NewEnumerator3
        (bind _outactors_4 (Actor|GetAllActorswithInterface "/Game/Blueprints/resetBtns/resetDrill_BPI.resetDrill_BPI_C"))
        (Class|ResetDrillBPI|ResetDrillStation(Message) _outactors_4)
        (Audio|PlaySound2D "/Engine/EditorSounds/GamePreview/EndPlayInEditor.EndPlayInEditor" 1.0 1.0 0.0 0 0)
        (Utilities|FlowControl|Delay 1.0)
        (Audio|PlaySound2D "/Game/G14_Assect/sfx/vo/VO/resetDrillStation.resetDrillStation" 1.0 1.0 0.0 0 0))
      (:NewEnumerator4
        (bind _outactors_5 (Actor|GetAllActorswithInterface "/Game/Blueprints/resetBtns/resetSoldering_BPI.resetSoldering_BPI_C"))
        (Class|ResetSolderingBPI|ResetSoldering(Message) _outactors_5)
        (Audio|PlaySound2D "/Engine/EditorSounds/GamePreview/EndPlayInEditor.EndPlayInEditor" 1.0 1.0 0.0 0 0)
        (Utilities|FlowControl|Delay 1.0)
        (Audio|PlaySound2D "/Game/G14_Assect/sfx/vo/VO/resetSolderStation.resetSolderStation" 1.0 1.0 0.0 0 0))
      (:NewEnumerator5
        (bind _outactors_6 (Actor|GetAllActorswithInterface "/Game/Blueprints/resetBtns/resetTestBed_BPI.resetTestBed_BPI_C"))
        (Class|ResetTestBedBPI|ResetTestBed(Message) _outactors_6)
        (Audio|PlaySound2D "/Engine/EditorSounds/GamePreview/EndPlayInEditor.EndPlayInEditor" 1.0 1.0 0.0 0 0))
      (:NewEnumerator6
        (CameraFades|StartCameraFade :self (Game|GetPlayerCameraManager 0) :ToAlpha 1.0 :Duration 4.0 :bShouldFadeAudio true :bHoldWhenFinished true)
        (Utilities|FlowControl|Delay 5.0)
        (Game|OpenLevel(byName) "endMap"))
      (:NewEnumerator7
        (CameraFades|StartCameraFade :self (Game|GetPlayerCameraManager 0) :ToAlpha 1.0 :Duration 4.0 :bShouldFadeAudio true :bHoldWhenFinished true)
        (Utilities|FlowControl|Delay 0.5)
        (Game|OpenLevel(byName) "quitMap"))
      (:NewEnumerator8
        (bind _outactors_7 (Actor|GetAllActorswithInterface "/Game/Blueprints/resetBtns/resetPractice_BPI.resetPractice_BPI_C"))
        (Class|ResetPracticeBPI|ResetPractice(Message) _outactors_7)
        (Audio|PlaySound2D "/Engine/EditorSounds/GamePreview/EndPlayInEditor.EndPlayInEditor" 1.0 1.0 0.0 0 0)
        (Utilities|FlowControl|Delay 3.0)
        (Audio|PlaySound2D "/Game/G14_Assect/sfx/vo/pickupPCB.pickupPCB" 1.0 1.0 0.0 0 0)
        (Utilities|FlowControl|Delay 5.0)
        (Audio|PlaySound2D "/Game/G14_Assect/sfx/vo/move2WShop.move2WShop" 1.0 1.0 0.0 0 0)))))

(event OnComponentBeginOverlap(textshowColider)
  (params (OverlappedComponent :type Primitive%20Component%20Object%20Reference) (OtherActor :type Actor%20Object%20Reference) (OtherComp :type Primitive%20Component%20Object%20Reference) (OtherBodyIndex :type Integer) (bFromSweep :type Boolean) (SweepResult :type Hit%20Result%20Structure%20%28by%20ref%29))
  ;[0.05303 1 0] Show/hide text code
  (bind _asvrpawn (Utilities|Casting|CastToVRPawn OtherActor))
  (if (Collision|IsOverlappingActor (Variables|Default|Gettext%20show%20Colider) _asvrpawn :!class /Script/Engine.PrimitiveComponent)
    (Rendering|SetVisibility (Variables|Default|GetCube1) true true)))

(event Collision|EventActorEndOverlap
  (params (OtherActor :type Actor%20Object%20Reference))
  ;[0.05303 1 0] Show/hide text code
  (bind _asvrpawn (Utilities|Casting|CastToVRPawn OtherActor))
  (if (not (Collision|IsOverlappingActor (Variables|Default|Gettext%20show%20Colider) _asvrpawn :!class /Script/Engine.PrimitiveComponent))
    (Rendering|SetVisibility (Variables|Default|GetCube1) false true)))

(event EventTick
  (params (DeltaSeconds :type Float%20%28single-precision%29))
  ;[0.06333 1 0] head tracking text
  (if (Variables|/Script/Engine.SceneComponent|GetbVisible (Variables|Default|GetCube1))
    (bind _asvrpawn (Utilities|Casting|CastToVRPawn (Game|Player|GetPlayerPawn 0)))
    (Transformation|SetWorldRotation (Variables|Default|GetCube1) (Math|Conversions|RotationFromXVector (Math|Vector|GetUnitDirection(Vector) (Transformation|GetWorldLocation (Variables|Default|GetCube1)) (Transformation|GetWorldLocation (Components|GetChildComponent (Variables|/Game/VRTemplate/Blueprints/VRPawn.VRPawn_C|GetCamera _asvrpawn) 0)))) false false)))

(fn ConstructionScript
  (Transformation|AddLocalOffset (Variables|Default|GetCube1) (Variables|Default|Gettext%20position%20offset) false false)
  (Rendering|Components|TextRender|SetText (Variables|Default|GetTextRender) (Utilities|Text|ToText(String) (Variables|Default|GetDisplay%20Text)))
  (Rendering|SetVisibility (Variables|Default|GetCube1) false true))