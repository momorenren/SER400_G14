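; A VR push button that resets an area by sending ResetMessage with its ResetArea value to actors implementing Reset_interface.
; Touching the switch collider with either hand sphere plays a sound and swaps the cylinder material for a one-second delay before the reset is sent.
; A text label, hidden at construction, shows while the VR pawn overlaps its collider and turns toward the player's camera each tick.
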(event OnComponentBeginOverlap(SwitchColider)
  (params (OverlappedComponent :type Primitive%20Component%20Object%20Reference) (OtherActor :type Actor%20Object%20Reference) (OtherComp :type Primitive%20Component%20Object%20Reference) (OtherBodyIndex :type Integer) (bFromSweep :type Boolean) (SweepResult :type Hit%20Result%20Structure%20%28by%20ref%29))
  (bind _switch_colider (Variables|Default|GetSwitch%20Colider))
  (bind _cylinder (Variables|Default|GetCylinder))
  ;[1 1 1] Press button things
  (bind _asvrpawn (Utilities|Casting|CastToVRPawn (Game|Player|GetPlayerPawn 0)))
  (if (or (Class|PrimitiveComponent|IsOverlappingComponent _switch_colider (Variables|/Game/VRTemplate/Blueprints/VRPawn.VRPawn_C|GetrightSphereCollider1 _asvrpawn)) (Class|PrimitiveComponent|IsOverlappingComponent _switch_colider (Variables|/Game/VRTemplate/Blueprints/VRPawn.VRPawn_C|GetleftSphereCollider _asvrpawn)))
    (Audio|PlaySound2D "/Engine/EditorSounds/GamePreview/EjectFromPlayer.EjectFromPlayer" 1.0 1.0 0.0 0 0)
    (Rendering|Material|SetMaterial _cylinder 0 "/Engine/EngineDebugMaterials/VertexColorViewMode_BlueOnly.VertexColorViewMode_BlueOnly")
    (Utilities|FlowControl|Delay 1.0)
    (Rendering|Material|SetMaterial _cylinder 0 "/Game/Blueprints/Soldering_iron/7_sement.7_sement")
    (bind _outactors (Actor|GetAllActorswithInterface "/Game/Interfaces/reset_interface.reset_interface_C"))
    (Class|ResetInterface|Reset(Message) _outactors (Variables|Default|Getreset%20area))))

(event OnComponentBeginOverlap(textshowColider)
  (params (OverlappedComponent :type Primitive%20Component%20Object%20Reference) (OtherActor :type Actor%20Object%20Reference) (OtherComp :type Primitive%20Component%20Object%20Reference) (OtherBodyIndex :type Integer) (bFromSweep :type Boolean) (SweepResult :type Hit%20Result%20Structure%20%28by%20ref%29))
  ;[0.05303 1 0] Show/hide text code
  (bind _asvrpawn (Utilities|Casting|CastToVRPawn OtherActor))
  (if (Collision|IsOverlappingActor (Variables|Default|Gettext%20show%20Colider) _asvrpawn :!class /Script/Engine.PrimitiveComponent)
    (Rendering|SetVisibility (Variables|Default|GetTextRender) true false)))

(event Collision|EventActorEndOverlap
  (params (OtherActor :type Actor%20Object%20Reference))
  ;[0.05303 1 0] Show/hide text code
  (bind _asvrpawn (Utilities|Casting|CastToVRPawn OtherActor))
  (if (not (Collision|IsOverlappingActor (Variables|Default|Gettext%20show%20Colider) _asvrpawn :!class /Script/Engine.PrimitiveComponent))
    (Rendering|SetVisibility (Variables|Default|GetTextRender) false false)))

(event EventTick
  (params (DeltaSeconds :type Float%20%28single-precision%29))
  ;[0.06333 1 0] head tracking text
  (if (Variables|/Script/Engine.SceneComponent|GetbVisible (Variables|Default|GetTextRender))
    (bind _asvrpawn (Utilities|Casting|CastToVRPawn (Game|Player|GetPlayerPawn 0)))
    (Transformation|SetWorldRotation (Variables|Default|GetTextRender) (Math|Conversions|RotationFromXVector (Math|Vector|GetUnitDirection(Vector) (Transformation|GetWorldLocation (Variables|Default|GetTextRender)) (Transformation|GetWorldLocation (Components|GetChildComponent (Variables|/Game/VRTemplate/Blueprints/VRPawn.VRPawn_C|GetCamera _asvrpawn) 0)))) false false)))

(fn ConstructionScript
  (Rendering|SetVisibility (Variables|Default|GetTextRender) false true))