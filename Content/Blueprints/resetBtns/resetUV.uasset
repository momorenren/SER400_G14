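; Reset button actor for the UV station, hidden with collision and tick off at start.
; A ResetStationResets event shows and enables it only when the station index is 2, and hides and disables it otherwise.
; On overlap it briefly swaps its cylinder material, sends ResetUVMessage to all actors implementing the Pcb2_hide_BPI interface, then plays two sounds a second apart.
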(event EventBeginPlay
  (Development|SetHiddeninGame (Variables|Default|GetDefaultSceneRoot) true true)
  (Collision|SetActorEnableCollision false)
  (Actor|Tick|SetActorTickEnabled false))

(event EventResetStationResets
  (params (stationIdx :type Integer))
  (bind _defaultsceneroot (Variables|Default|GetDefaultSceneRoot))
  (Math|Integer|CompareInt stationIdx 2
    (:>
      (Development|SetHiddeninGame _defaultsceneroot true true :!label _label)
      (Collision|SetActorEnableCollision false)
      (Actor|Tick|SetActorTickEnabled false))
    (:==
      (Development|SetHiddeninGame _defaultsceneroot false true)
      (Collision|SetActorEnableCollision true)
      (Actor|Tick|SetActorTickEnabled true))
    (:<
      (goto _label))))

(event EventTick
  (params (DeltaSeconds :type Float%20%28single-precision%29)))

(event Collision|EventActorBeginOverlap
  (params (OtherActor :type Actor%20Object%20Reference))
  (bind _cylinder (Variables|Default|GetCylinder))
  (Rendering|Material|SetMaterial _cylinder 0 "/Engine/EngineDebugMaterials/VertexColorViewMode_BlueOnly.VertexColorViewMode_BlueOnly")
  (Utilities|FlowControl|Delay 0.5)
  (Rendering|Material|SetMaterial _cylinder 0 "/Game/BluePrints/Soldering_iron/7_sement.7_sement")
  (bind _outactors (Actor|GetAllActorswithInterface "/Game/pcb/pcb2/pcb2/Geometries/pcb2_hide_BPI.pcb2_hide_BPI_C"))
  (Class|ResetUVBPI|ResetUV(Message) _outactors)
  (Audio|PlaySound2D "/Engine/EditorSounds/GamePreview/EndPlayInEditor.EndPlayInEditor" 1.0 1.0 0.0 0 0)
  (Utilities|FlowControl|Delay 1.0)
  (Audio|PlaySound2D "/Game/G14_Assect/sfx/vo/VO/resetUVStation.resetUVStation" 1.0 1.0 0.0 0 0))

(fn ConstructionScript)