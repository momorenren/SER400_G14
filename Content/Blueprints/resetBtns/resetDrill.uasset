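; Reset button actor that triggers a drill station reset when another actor overlaps it.
; Its cylinder flashes a blue material for half a second, then returns to the cement material.
; It then sends ResetDrillStationMessage to actors implementing ResetDrill_BPI, prints a debug index and plays a sound.
; Disconnected leftovers include tag-based actor lookups, a direct reset call and a loop over the interface actors.
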(event EventBeginPlay)

(event EventTick
  (params (DeltaSeconds :type Float%20%28single-precision%29)))

(event Collision|EventActorBeginOverlap
  (params (OtherActor :type Actor%20Object%20Reference))
  (bind _cylinder (Variables|Default|GetCylinder))
  (Rendering|Material|SetMaterial _cylinder 0 "/Engine/EngineDebugMaterials/VertexColorViewMode_BlueOnly.VertexColorViewMode_BlueOnly")
  (Utilities|FlowControl|Delay 0.5)
  (Rendering|Material|SetMaterial _cylinder 0 "/Game/Blueprints/Soldering_iron/7_sement.7_sement")
  (bind _outactors (Actor|GetAllActorswithInterface "/Game/Blueprints/resetBtns/resetDrill_BPI.resetDrill_BPI_C"))
  (Class|ResetDrillBPI|ResetDrillStation(Message) _outactors)
  (Development|PrintString (Utilities|String|ToString(Integer) (stale _array_index)) true true "(R=0.000000,G=0.165000,B=0.250000,A=1.000000)" 4.0)
  (Audio|PlaySound2D "/Engine/EditorSounds/GamePreview/EndPlayInEditor.EndPlayInEditor" 1.0 1.0 0.0 0 0))

(fn ConstructionScript)