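; PCB actor for the chemical station, apparently the board coming from the UV step, which disappears when the tong touches it.
; BeginPlay stores the mesh's world transform, and an overlap between its collider and a Tong_PCB hides the whole actor.
; ResetChemical restores the stored transform and unhides it.
; GetPcbState exposes the board's state, while GivePcb is an empty stub.
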(event OnComponentBeginOverlap(PCB_UV_collider)
  (params (OverlappedComponent :type Primitive%20Component%20Object%20Reference) (OtherActor :type Actor%20Object%20Reference) (OtherComp :type Primitive%20Component%20Object%20Reference) (OtherBodyIndex :type Integer) (bFromSweep :type Boolean) (SweepResult :type Hit%20Result%20Structure%20%28by%20ref%29))
  ;[0.1779 0.2677 1] PCB_UV overlaps with tong
  (Utilities|Casting|CastToTong_PCB OtherActor)
  (Rendering|SetActorHiddenInGame true))

(event EventResetChemical
  ;[1 1 1] Reset chemical station
  (Transformation|SetWorldTransform (Variables|Default|GetPCB_Static_Mesh) (Variables|Default|GetPCB_UV_trans_var) false false)
  (Rendering|SetActorHiddenInGame false))

(event EventBeginPlay
  ;[1 0.108 0.3355] Record initial transform
  (Variables|Default|SetPCB_UV_trans_var (Transformation|GetWorldTransform (Variables|Default|GetPCB_Static_Mesh))))

(fn ConstructionScript)

(fn GivePcb
  (return 0))

(fn GetPcbState
  (return (Variables|Default|Getthis_pcb_state)))