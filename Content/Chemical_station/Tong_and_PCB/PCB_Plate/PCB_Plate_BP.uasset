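; PCB plate in the chemical station that reacts when the tong holding the PCB reaches it, completing the station and pointing to drilling.
; On overlap with a Tong_PCB, it plays plate audio, reveals the drill-ready PCB found at BeginPlay, and swaps its voiceover for the station-done line.
; Interface broadcasts switch the instruction texts and show the Pcb4 message.
; ResetChemical hides the drill-ready PCB and that message again.
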(event OnComponentBeginOverlap(PCB_Plate_collider)
  (params (OverlappedComponent :type Primitive%20Component%20Object%20Reference) (OtherActor :type Actor%20Object%20Reference) (OtherComp :type Primitive%20Component%20Object%20Reference) (OtherBodyIndex :type Integer) (bFromSweep :type Boolean) (SweepResult :type Hit%20Result%20Structure%20%28by%20ref%29))
  (Utilities|Casting|CastToTong_PCB OtherActor)
  (Audio|Components|Audio|Play (Variables|Default|Getplate_audio) 0.0)
  (Rendering|SetActorHiddenInGame (Variables|Default|GetPCB_ready_drillVR) false)
  (bind _outactors (Actor|GetAllActorswithInterface "/Game/Chemical_station/chemical_text/Chemical_text_interface.Chemical_text_interface_C"))
  (Class|ChemicalTextInterface|TakePCBOutTextHide(Message) _outactors)
  (Class|ChemicalTextInterface|MovetoDrillTextShow(Message) _outactors)
  ;[1 1 1] dw's
  (CallFunction|KillSound)
  (bind _returnvalue (Audio|SpawnSound2D "/Game/G14_Assect/sfx/vo/VO/Chem_station_done.Chem_station_done" 1.0 1.0 0.0 0))
  (Variables|Default|SetvoPlaying _returnvalue)
  (bind _outactors_2 (Actor|GetAllActorswithInterface "/Game/pcb/pcb4/pcb4/Geometries/pcb4_show_BPI.pcb4_show_BPI_C"))
  (Class|Pcb4ShowBPI|ShowPcb4(Message) _outactors_2))

(event EventBeginPlay
  (bind _returnvalue (Actor|GetActorOfClass "/Game/Chemical_station/Tong_and_PCB/PCBs_of_Chemical/PCB_Ready_DrillBP.PCB_Ready_DrillBP_C"))
  (bind _output_get (Variables|Default|SetPCB_ready_drillVR _returnvalue))
  (Utilities|Casting|CastToPCB_Ready_DrillBP _output_get))

(event Collision|EventActorBeginOverlap
  (params (OtherActor :type Actor%20Object%20Reference)))

(event EventTick
  (params (DeltaSeconds :type Float%20%28single-precision%29)))

(event EventResetChemical
  (Rendering|SetActorHiddenInGame (Variables|Default|GetPCB_ready_drillVR) true)
  (bind _outactors (Actor|GetAllActorswithInterface "/Game/pcb/pcb4/pcb4/Geometries/pcb4_show_BPI.pcb4_show_BPI_C"))
  (Class|Pcb4ShowBPI|HiddenPcb4(Message) _outactors))

(fn ConstructionScript)

(fn KillSound
  (bind _voplaying (Variables|Default|GetvoPlaying))
  (if (Utilities|IsValid _voplaying)
    (Components|Activation|SetActive _voplaying false false)))